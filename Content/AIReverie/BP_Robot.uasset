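; BP_Robot is an automated robot that moves on a timer and captures and records viewport data after each move.
; BeginPlay starts a looping timer at the SecondsBetweenMoves interval, and EndPlay clears it.
; Each tick of that timer calls MoveForward, rotates only if the forward move fails, then calls CaptureAndRecordViewportData in either case.
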(event Custom|OnPerformMove
  (bind _returnvalue (Class|RobotPawn|MoveForward))
  (if (not _returnvalue)
    (Class|RobotPawn|Rotate))
  (Class|RobotPawn|CaptureandRecordViewportData))

(event EventBeginPlay
  (bind _returnvalue (Utilities|Time|SetTimerbyEvent (delegate Custom|OnPerformMove) (Variables|Default|GetSecondsBetweenMoves) true))
  (Variables|Default|SetMovementTimerHandle _returnvalue))

(event EventEndPlay
  (params (EndPlayReason :type EEndPlayReason%20Enum :default "Destroyed"))
  (Utilities|Time|ClearandInvalidateTimerbyHandle (Variables|Default|GetMovementTimerHandle)))

(fn ConstructionScript)